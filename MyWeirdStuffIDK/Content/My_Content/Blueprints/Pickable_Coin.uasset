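; Pickable coin actor that spins continuously and adds a random value to the ThirdPersonCharacter's Coins when touched.
; On BeginPlay, SetCoinAmount rolls the value, scales the mesh by it and, above one, scatters extra runtime-spawned meshes inside the sphere.
; Sphere overlap disables collision, credits the player and plays a pickup sound.
; A timeline then animates the coin's height before an explosion effect, sound and actor destruction.
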(event OnComponentBeginOverlap(Sphere)
  (params (OverlappedComponent :type Primitive%20Component%20Object%20Reference) (OtherActor :type Actor%20Object%20Reference) (OtherComp :type Primitive%20Component%20Object%20Reference) (OtherBodyIndex :type Integer) (bFromSweep :type Boolean) (SweepResult :type Hit%20Result%20Structure%20%28by%20ref%29))
  (bind _coin_model (Variables|Default|GetCoin%20model))
  (bind _returnvalue (Transformation|GetWorldLocation _coin_model))
  ;[1 0.9839 0.349] Overlapp box collsion (coin) events
  (if (== (Utilities|GetClass OtherActor) "/Game/ThirdPersonBP/Blueprints/ThirdPersonCharacter.ThirdPersonCharacter_C")
    ;;[1 1 1] Update player coins value
    (Collision|SetActorEnableCollision false)
    (bind _asthird_person_character (Utilities|Casting|CastToThirdPersonCharacter OtherActor))
    (Variables|/Game/ThirdPersonBP/Blueprints/ThirdPersonCharacter.ThirdPersonCharacter_C|SetCoins _asthird_person_character (+ (Variables|/Game/ThirdPersonBP/Blueprints/ThirdPersonCharacter.ThirdPersonCharacter_C|GetCoins _asthird_person_character) (Variables|Default|GetAmount)))
    (Audio|PlaySoundatLocation "/Game/My_Content/Audio/135936__bradwesson__collectcoin_EDITED.135936__bradwesson__collectcoin_EDITED" (Transformation|GetWorldLocation OverlappedComponent) "0, 0, 0" 1.0 1.0 0.0 0 0 0 0)
    ;;;[0.3694 0.2833 1] Playing the destroy animation and then actually destroying the actor
    (Components|Timeline|SetPlayRate (Variables|Default|GetT_IdleAnimation) 3.5)
    (bind _newzobjectlocationvalue (Timeline|T_IdleAnimation PlayFromStart)
      (:Update
        (Transformation|SetRelativeLocation _coin_model (Math|Vector|MakeVector 0.0 0.0 _newzobjectlocationvalue) false false))
      (:Finished
        (Effects|SpawnEmitteratLocation "/Game/StarterContent/Particles/P_Explosion.P_Explosion" _returnvalue)
        (Audio|PlaySoundatLocation "/Game/StarterContent/Audio/Explosion_Cue.Explosion_Cue" _returnvalue "0, 0, 0" 0.6 1.0 0.0 0 0 0 0)
        (Actor|DestroyActor)))))

(event EventBeginPlay
  (bind _t_rotationanim (Variables|Default|GetT_RotationAnim))
  ;[1 1 1] Begin play events
  (Utilities|FlowControl|Sequence
    (:then_0
      ;;[1 1 1] Calling "Set coin amount" function
      (bind _amount (CallFunction|SetCoinAmount (Variables|Default|GetCoin%20model)))
      (Variables|Default|SetAmount _amount))
    (:then_1
      ;;[0.388 0.2656 1] Playing the rotation animation and looping it
      (Components|Timeline|SetPlayRate _t_rotationanim 4.0)
      (Components|Timeline|SetLooping _t_rotationanim true)
      (bind _z_rotationvalue (Timeline|T_RotationAnim PlayFromStart)
        (:Update
          (Transformation|SetRelativeRotation (Variables|Default|GetCoin%20model) (Math|Rotator|MakeRotator 0.0 0.0 _z_rotationvalue) false false))))))

(fn ConstructionScript)

(fn SetCoinAmount
  (params (Mesh%20object :type Static%20Mesh%20Component%20Object%20Reference))
  (bind _sphere (Variables|Default|GetSphere))
  ;[1 1 1] Function for get one number between 1 and 3, then scale the mesh relative to the random number
  (bind _output_get (LocalVariables|SetLocal%20random%20value (Math|Random|RandomIntegerinRange 1 3)))
  (Utilities|FlowControl|Sequence
    (:then_0
      (if (== _output_get 1)
        ;;[1 1 1] Number is one?, If is it the case, add one to the scale
        (bind _result (Math|Float|IncrementFloat (Math|Conversions|ToFloat(Integer) (LocalVariables|GetLocal%20random%20value)))
          (:%20%20
            (Transformation|SetRelativeScale3D Mesh%20object (Math|Vector|MakeVector _result _result _result))))
        (else
          (Transformation|SetRelativeScale3D Mesh%20object (Math|Vector|MakeVector (Math|Conversions|ToFloat(Integer) (LocalVariables|GetLocal%20random%20value)) (Math|Conversions|ToFloat(Integer) (LocalVariables|GetLocal%20random%20value)) (Math|Conversions|ToFloat(Integer) (LocalVariables|GetLocal%20random%20value)))))))
    (:then_1
      ;;[1 1 1] Add more meshes depending of the amount to give
      (if (!= (LocalVariables|GetLocal%20random%20value) 1)
        (for _index (range 0 (- (LocalVariables|GetLocal%20random%20value) 1))
          (bind _returnvalue (AddComponent|AddStaticMeshComponent false (Math|Transform|MakeTransform (Math|Random|RandomPointinBoundingBox (Variables|/Script/Engine.SceneComponent|GetRelativeLocation _sphere) (Math|Conversions|ToVector(Float) (/ (Components|Sphere|GetScaledSphereRadius _sphere) 2.0))) "0,0.000000, 0")))
          (Transformation|AttachComponentToComponent _returnvalue (Variables|Default|GetCoin%20model) "None" "KeepWorld" "KeepWorld" "KeepWorld" true))))
    (:then_2
      (return _output_get))))