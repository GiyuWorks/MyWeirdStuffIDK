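; BP_Door is a teleport door that opens on overlap and presents a teleport menu.
; Begin overlap plays the door and light sequences, reveals the transport cube, zeroes the character's walk speed, and swaps all widgets for Teleport_Widget with UI-only input.
; End overlap reverses the door, hides the effects if the light sequence is playing, and restores the controllers widget passed in through Callcontrollerswidget unless it was destroyed.
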(event OnComponentBeginOverlap(Collision)
  (params (OverlappedComponent :type Primitive%20Component%20Object%20Reference) (OtherActor :type Actor%20Object%20Reference) (OtherComp :type Primitive%20Component%20Object%20Reference) (OtherBodyIndex :type Integer) (bFromSweep :type Boolean) (SweepResult :type Hit%20Result%20Structure%20%28by%20ref%29))
  (bind _returnvalue (Game|GetPlayerController 0))
  ;[1 1 1] Door open events
  (Utilities|FlowControl|Sequence
    (:then_0
      (if (not (Variables|Default|GetDoor%20is%20open?))
        (Sequencer|Player|Play (Variables|/Script/ActorSequence.ActorSequenceComponent|GetSequencePlayer (Variables|Default|GetOpen_Anim)) :!class /Script/MovieScene.MovieSceneSequencePlayer)
        (Variables|Default|SetDoor%20is%20open? true)
        (Rendering|SetVisibility (Variables|Default|GetDoor_Light) true false)
        (Sequencer|Player|Play (Variables|/Script/ActorSequence.ActorSequenceComponent|GetSequencePlayer (Variables|Default|GetLight_Anim)) :!class /Script/MovieScene.MovieSceneSequencePlayer)
        (Utilities|FlowControl|Delay 0.5)
        (Rendering|SetVisibility (Variables|Default|GetTransport_cube) true false)))
    (:then_1
      ;;[1 1 1] Setting input mode to only UI
      (Variables|/Script/Engine.PlayerController|SetbShowMouseCursor _returnvalue true)
      (Input|SetInputModeUIOnly _returnvalue 0 "DoNotLock")
      (bind _asthird_person_character (Utilities|Casting|CastToThirdPersonCharacter OtherActor))
      (Variables|/Script/Engine.CharacterMovementComponent|SetMaxWalkSpeed (Variables|/Script/Engine.Character|GetCharacterMovement _asthird_person_character) 0.0)
      (Viewport|RemoveAllWidgets)
      (UserInterface|Viewport|AddtoViewport (Variables|Default|GetTransport%20widget) 0))))

(event OnComponentEndOverlap(Collision)
  (params (OverlappedComponent :type Primitive%20Component%20Object%20Reference) (OtherActor :type Actor%20Object%20Reference) (OtherComp :type Primitive%20Component%20Object%20Reference) (OtherBodyIndex :type Integer))
  (bind _light_anim (Variables|Default|GetLight_Anim))
  (bind _transport_cube (Variables|Default|GetTransport_cube))
  (bind _sequenceplayer (Variables|/Script/ActorSequence.ActorSequenceComponent|GetSequencePlayer _light_anim))
  ;[1 1 1] Door close events
  (Utilities|FlowControl|Sequence
    (:then_0
      (if (Variables|Default|GetDoor%20is%20open?)
        (Class|MovieSceneSequencePlayer|PlayReverse (Variables|/Script/ActorSequence.ActorSequenceComponent|GetSequencePlayer (Variables|Default|GetOpen_Anim)))
        (if (Audio|Components|Audio|IsPlaying _sequenceplayer)
          (Sequencer|Player|Stop _sequenceplayer :!class /Script/MovieScene.MovieSceneSequencePlayer)
          (Variables|Default|SetDoor%20is%20open? false)
          (Rendering|SetVisibility (Variables|Default|GetDoor_Light) false false)
          (if (Rendering|IsVisible _transport_cube)
            (Rendering|SetVisibility _transport_cube false false)))))
    (:then_1
      ;;[1 1 1] Communicating with Level blueprint and getting the controllers widget variable on it
      (bind _ascontrollers_widget (Utilities|Casting|CastToControllers_Widget (stale Custom|Call%20controllers%20widget _output_get)))
      (if (not (Variables|/Game/My_Content/HUD/Controllers_Widget.Controllers_Widget_C|GetWidget%20was%20destroyed? _ascontrollers_widget))
        (UserInterface|Viewport|AddtoViewport _ascontrollers_widget 0)))))

(event Custom|Call%20controllers%20widget
  (params (Controllers :type Controllers%20Widget%20Object%20Reference))
  ;[1 1 1] Door close events
  ;;[1 1 1] Communicating with Level blueprint and getting the controllers widget variable on it
  (bind _output_get (Variables|Default|SetControllers%20widget Controllers)))

(event EventBeginPlay
  ;[1 1 1] Begin play events
  (Utilities|FlowControl|Sequence
    (:then_0
      (Rendering|SetVisibility (Variables|Default|GetDoor_Light) false false)
      (Variables|Default|SetRandom_Number (Math|Random|RandomInteger 10)))
    (:then_1
      ;;[1 1 1] Making frame and door one with an a array
      (Variables|Default|SetFire (Variables|Default|GetParticleSystem))
      (Variables|Default|SetMesh_Door (Utilities|Array|MakeArray (Variables|Default|GetFrame_Door) (Variables|Default|GetDoor))))
    (:then_2
      (bind _returnvalue (UserInterface|CreateWidget "/Game/My_Content/HUD/Teleport_Widget.Teleport_Widget_C" (Game|GetPlayerController 0)))
      (Variables|Default|SetTransport%20widget _returnvalue))))

(fn ConstructionScript)